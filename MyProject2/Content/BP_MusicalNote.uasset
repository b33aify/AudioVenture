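; BP_MusicalNote is a pickup actor for a musical note that the third-person character collects by overlapping it.
; On overlap it adds its NoteSound to the character's CollectedNotes, plays that sound at its location and destroys itself.
; BeginPlay assigns AssignedNiagara to the NiagaraEffect variable.
; A DestroyComponent call on the effect is left unconnected and never runs.
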(event `self.ReceiveActorBeginOverlap`
  (params (OtherActor :type "Actor Object Reference"))
  (bind _notesound (`self.NoteSound`))
  (bind _asbp_third_person_character (cast `/Game/ThirdPerson/Blueprints/BP_ThirdPersonCharacter` OtherActor))
  (`KismetArrayLibrary.Array_Add` (`/Game/ThirdPerson/Blueprints/BP_ThirdPersonCharacter.CollectedNotes` _asbp_third_person_character) _notesound)
  (`GameplayStatics.PlaySoundAtLocation` _notesound (`self.K2_GetActorLocation`) (struct) 1.0 1.0 0.0 null null null null)
  (`self.K2_DestroyActor`))

(event `self.ReceiveBeginPlay`
  (bind _output_get (set `self.NiagaraEffect` (`self.AssignedNiagara`))))

(fn `UserConstructionScript`)